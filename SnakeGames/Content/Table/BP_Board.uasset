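; BP_Board is the board actor for a snakes-style tile game, generating the grid and moving the player across it.
; On BeginPlay, nested loops spawn BP_Tile actors into TileList, offsetting odd columns in Y for a staggered layout.
; Inside that loop it also hands itself to BP_Player and spawns BP_Snakes linking tile pairs from the Snakes map.
; MovePlayer moves the player pawn to an indexed tile's location.
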(event `self.ReceiveBeginPlay`
  (bind _snakes (`self.Snakes`))
  ;[1 1 1] Spawn Tiles
  (for _index (range (+ (`self.Grid X`) 1))
    (for _index_2 (range (+ (`self.Grid Y`) 1))
      (bind _returnvalue (* _index (`self.Spacing X`)))
      (bind _returnvalue_2 (* _index_2 (`self.Spacing Y`)))
      (bind _returnvalue_3 (`|SpawnActorFromClass` "/Game/Table/BP_Tile.BP_Tile_C" (`KismetMathLibrary.MakeTransform` (`KismetMathLibrary.SelectVector` (`KismetMathLibrary.MakeVector` _returnvalue _returnvalue_2) (`KismetMathLibrary.MakeVector` _returnvalue (+ (`self.Offset`) _returnvalue_2)) (== (mod _index 2) 0)) (struct)) "Undefined" "OverrideRootScale" null null))
      (`KismetArrayLibrary.Array_Add` (`self.TileList`) _returnvalue_3)
      (set `/Game/Player/BP_PLayer.BoardRef` self (cast `/Game/Player/BP_PLayer` (`GameplayStatics.GetPlayerPawn` 0) :!pure true))
      (bind _keys (`BlueprintMapLibrary.Map_Keys` _snakes))
      (for (_array_element _array_index) _keys
        (bind _values (`BlueprintMapLibrary.Map_Values` _snakes))
        (bind _returnvalue_4 (`|SpawnActorFromClass` "/Game/Snake/BP_Snake.BP_Snake_C" (`KismetMathLibrary.MakeTransform` (0.0 0.0 0.0)) "Undefined" "OverrideRootScale" null null))
        (`/Game/Snake/BP_Snake.Define` _returnvalue_4 (`|GetArrayItem` (`self.TileList`) _array_element) (`|GetArrayItem` (`self.TileList`) (`|GetArrayItem` _values _array_index)))))))

(fn `MovePlayer`
  (params (Index :type Integer))
  (`self.K2_SetActorLocation` (`GameplayStatics.GetPlayerPawn` 0) (`SceneComponent.K2_GetComponentLocation` (`Actor.RootComponent` (`|GetArrayItem` (`self.TileList`) Index))) false false))

(fn `UserConstructionScript`)