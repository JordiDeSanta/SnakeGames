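; Player Blueprint for a dice board game that starts on the board's first tile, spawns a die and offers clamped spring-arm zoom.
; A left click throws the physics die once, and Tick waits until its velocity is zero.
; The die then teleports below the camera, a Trigger overlap with its face components sets the result, and Move passes the clamped tile index to the board before the die is destroyed.
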(event `InputAction|ZoomOut`
  (params (Key :type "Key Structure"))
  (bind _springarm (`self.SpringArm`))
  ;[1 1 1] Camera Zoom
  (:`Pressed`
    (set `SpringArmComponent.TargetArmLength` (`KismetMathLibrary.FClamp` (+ (`SpringArmComponent.TargetArmLength` _springarm) (`self.ZoomVelocity`)) 3000.0 10000.0) _springarm)))

(event `InputAction|ZoomIn`
  (params (Key :type "Key Structure"))
  (bind _springarm (`self.SpringArm`))
  ;[1 1 1] Camera Zoom
  (:`Pressed`
    (set `SpringArmComponent.TargetArmLength` (`KismetMathLibrary.FClamp` (- (`SpringArmComponent.TargetArmLength` _springarm) (`self.ZoomVelocity`)) 3000.0 10000.0) _springarm)))

(event `SpawnDice`
  (bind _returnvalue (`|SpawnActorFromClass` "/Game/Dice/BP_Dice.BP_Dice_C" (`KismetMathLibrary.MakeTransform` (`SceneComponent.K2_GetComponentLocation` (`self.Scene`)) (struct) (4.0 4.0 4.0)) "Undefined" "OverrideRootScale" null null))
  (set `self.DiceRef` _returnvalue))

(event `self.ReceiveBeginPlay`
  ;[1 1 1] Setting Spawm
  (`self.K2_SetActorLocation` (`self.K2_GetActorLocation` (`|GetArrayItem` (`/Game/Table/BP_Board.TileList` (`self.BoardRef`)))))
  (`self.SpawnDice`))

(event `Key|LeftMouseButton`
  (params (Key :type "Key Structure"))
  ;[1 1 1] Movement
  (:`Pressed`
    (`self.ThrowDice`)))

(event `ThrowDice`
  (bind _diceref (`self.DiceRef`))
  ;[1 1 1] Throw Dice
  (`/Engine/EditorBlueprintResources/StandardMacros.DoOnce` false :!label _label
    (:`Completed`
      (`PrimitiveComponent.SetSimulatePhysics` (`/Game/Dice/BP_Dice.StaticMesh` _diceref) true)
      (`ActorComponent.Deactivate` (`/Game/Dice/BP_Dice.RotatingMovement` _diceref))
      (`/Game/Dice/BP_Dice.Throw` (`self.DiceRef`))
      (`KismetSystemLibrary.Delay` 2.0))))

(event `self.ReceiveTick`
  (params (DeltaSeconds :type "Float (single-precision)"))
  ;[1 1 1] Checking
  (`/Engine/EditorBlueprintResources/StandardMacros.IsValid` (`self.DiceRef`)
    (:`Is Valid`
      (if (and (`/Game/Dice/BP_Dice.Throwed` (`self.DiceRef`)) (== (`KismetMathLibrary.VSize` (`SceneComponent.GetComponentVelocity` (`/Game/Dice/BP_Dice.StaticMesh` (`self.DiceRef`)))) 0.0))
        (`/Game/Dice/BP_Dice.Quiet` (`self.DiceRef`))
        (set `PrimitiveComponent.bGenerateOverlapEvents` true (`self.Trigger`))
        (`self.ShowDice`)
        (`KismetSystemLibrary.Delay` 2.0)
        (`self.Move` (`self.Result`))
        (set `PrimitiveComponent.bGenerateOverlapEvents` false (`self.Trigger`))
        (`self.Reset`)
        (`self.K2_DestroyActor` (`self.DiceRef`))))))

(event `Reset`
  ;[1 1 1] Throw Dice
  (goto _label :!via `Reset`))

(event `ShowDice`
  (bind (_returnvalue_x _returnvalue_y _returnvalue_z) (`KismetMathLibrary.BreakVector` (`SceneComponent.GetSocketLocation` (`self.SpringArm`) "SpringEndpoint")))
  ;[1 1 1] Show Result
  (`SceneComponent.K2_SetWorldLocation` (`/Game/Dice/BP_Dice.StaticMesh` (`self.DiceRef`)) (`KismetMathLibrary.MakeVector` _returnvalue_x _returnvalue_y (- _returnvalue_z 1000.0)) false true))

(event `self.Trigger.OnComponentBeginOverlap`
  (params (OverlappedComponent :type "PrimitiveComponent Object Reference") (OtherActor :type "Actor Object Reference") (OtherComp :type "PrimitiveComponent Object Reference") (OtherBodyIndex :type Integer) (bFromSweep :type Boolean) (SweepResult :type "HitResult Structure (by ref)"))
  ;[1 1 1] Result
  (bind _asbp_dice (cast `/Game/Dice/BP_Dice` OtherActor))
  (if (== (`/Game/Dice/BP_Dice.Six` _asbp_dice) OtherComp)
    (set `self.Result` 6)
    (elif (== (`/Game/Dice/BP_Dice.Five` _asbp_dice) OtherComp)
      (set `self.Result` 5)
      (elif (== (`/Game/Dice/BP_Dice.Four` _asbp_dice) OtherComp)
        (set `self.Result` 4)
        (elif (== (`/Game/Dice/BP_Dice.Three` _asbp_dice) OtherComp)
          (set `self.Result` 3)
          (elif (== (`/Game/Dice/BP_Dice.Two` _asbp_dice) OtherComp)
            (set `self.Result` 2)
            (elif (== (`/Game/Dice/BP_Dice.One` _asbp_dice) OtherComp)
              (set `self.Result` 1))))))))

(fn `Move`
  (params (n :type Integer))
  (`KismetSystemLibrary.PrintString` (`KismetStringLibrary.Conv_IntToString` n))
  (bind _output_get (set `self.TileIndex` (`KismetMathLibrary.Clamp` (+ n (`self.TileIndex`)) 0 (`/Game/Table/BP_Board.TileMax` (`self.BoardRef`)))))
  (`/Game/Table/BP_Board.MovePlayer` (`self.BoardRef`) _output_get))

(fn `UserConstructionScript`)